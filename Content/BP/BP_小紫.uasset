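; BP_小紫 is a player-controlled pawn that moves and interacts with nearby actors through Enhanced Input.
; BeginPlay adds the IMC_輸入管理器 mapping context, and IA_移動 drives movement along fixed world X and Y axes.
; IA_互動 sends the BPI_互動 interface message to every implementing actor overlapping 互動區域.
; 開始互動 then sets 是否互動, which blocks movement; this graph never clears it.
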(event Custom|開始互動
  (Variables|Default|Set是否互動 true))

(event Input|EnhancedActionEvents|EnhancedInputActionIA_互動
  (params (ActionValue :type Boolean) (ElapsedSeconds :type Float%20%28double-precision%29) (TriggeredSeconds :type Float%20%28double-precision%29) (InputAction :type Input%20Action%20Object%20Reference :default "/Game/輸入/IA_互動.IA_互動"))
  (:Started
    (for _array_element (Collision|GetOverlappingActors (Variables|Default|Get互動區域) 0 :!class /Script/Engine.PrimitiveComponent) ; 迴圈執行
      (if (Utilities|DoesObjectImplementInterface _array_element "/Game/BP/BPI_互動.BPI_互動_C")
        (Class|BPI互動|互動(Message) _array_element)
        (CallFunction|開始互動)))))

(event Input|EnhancedActionEvents|EnhancedInputActionIA_移動
  (params (ActionValue :type Vector%202D%20Structure) (ElapsedSeconds :type Float%20%28double-precision%29) (TriggeredSeconds :type Float%20%28double-precision%29) (InputAction :type Input%20Action%20Object%20Reference :default "/Game/輸入/IA_移動.IA_移動"))
  (:Triggered
    (if (not (Variables|Default|Get是否互動))
      (Pawn|Input|AddMovementInput "0.000000,1.000000,0.000000" (.Y (Math|Vector2D|BreakVector2D ActionValue)) false) ; 添加移動輸入
      (Pawn|Input|AddMovementInput "1.000000,0.000000,0.000000" (.X (Math|Vector2D|BreakVector2D ActionValue)) false) ; 添加移動輸入
    )))

(event EventBeginPlay
  (Input|AddMappingContext (PlayerController|LocalPlayerSubsystems|GetEnhancedInputLocalPlayerSubsystem (Game|GetPlayerController 0)) "/Game/輸入/IMC_輸入管理器.IMC_輸入管理器" 0 "(bIgnoreAllPressedKeysUntilRelease=True,bForceImmediately=False,bNotifyUserSettings=False)") ; 添加綁定環境
)

(fn ConstructionScript)